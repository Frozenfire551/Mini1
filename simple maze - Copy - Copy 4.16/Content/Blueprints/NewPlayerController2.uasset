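; Player controller for a two-player turn-based bomb game that alternates one controller between the Player1 and Player2 pawns.
; Enter triggers the current pawn's bombs, calls PlayerDie on the opponent, then possesses the pawn chosen by Player1Turn.
; Each handover refills that pawn's movement spaces and clears direction state on Plane actors; BeginPlay starts with Player1.
; Test duplicates the possession switch without the Plane reset and is not called here.
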(event EventTick
  (params (DeltaSeconds :type Float%20%28single-precision%29)))

(event EventBeginPlay
  (Utilities|FlowControl|Delay 0.2)
  (bind _outactors (Actor|GetAllActorsOfClass "/Game/FirstPersonBP/Blueprints/player1.player1_C"))
  (Pawn|Possess (Utilities|Array|Get(acopy) _outactors))
  (Variables|Default|Setplayer1Turn false)
  (bind _asplayer_1 (Utilities|Casting|CastToplayer1 (Game|Player|GetPlayerPawn 0)))
  (Variables|/Game/FirstPersonBP/Blueprints/player1.player1_C|Setspacesleft _asplayer_1 3)
  (Variables|Default|SetplaneCurrentPlace 0)
  (bind _outactors_2 (Actor|GetAllActorsOfClass "/Game/plane.plane_C"))
  (Variables|/Game/plane.plane_C|Setdirection%20to%20leave (Utilities|Array|Get(acopy) _outactors_2 (Variables|Default|GetplaneCurrentPlace)) "null" :!label _label)
  (Variables|/Game/plane.plane_C|Setway%20the%20player%20came%20in (Utilities|Array|Get(acopy) _outactors_2 (Variables|Default|GetplaneCurrentPlace)) "null")
  (if (not (== (Variables|Default|GetplaneCurrentPlace) (Utilities|Array|Length _outactors_2)))
    (Math|Integer|IncrementInt (Variables|Default|GetplaneCurrentPlace)
      (:%20%20
        (goto _label)))))

(event Input|KeyboardEvents|Enter
  (params (Key :type Key%20Structure))
  (bind _returnvalue (Game|GetPlayerCharacter 0))
  (:Pressed
    (Utilities|FlowControl|Delay 0.2)
    (bind _asplayer_1 (Utilities|Casting|CastToplayer1 _returnvalue)
      (:then
        (Default|TriggerBombs _asplayer_1)
        (bind _outactors (Actor|GetAllActorsOfClass "/Game/FirstPersonBP/Blueprints/player2.player2_C"))
        (Default|PlayerDie? (Utilities|Array|Get(acopy) _outactors)))
      (:CastFailed
        (bind _asplayer_2 (Utilities|Casting|CastToplayer2 _returnvalue))
        (Default|TriggerBombs _asplayer_2)
        (bind _outactors_2 (Actor|GetAllActorsOfClass "/Game/FirstPersonBP/Blueprints/player1.player1_C"))
        (Default|PlayerDie? (Utilities|Array|Get(acopy) _outactors_2))))
    (if (Variables|Default|Getplayer1Turn)
      (bind _outactors_3 (Actor|GetAllActorsOfClass "/Game/FirstPersonBP/Blueprints/player1.player1_C"))
      (Pawn|Possess (Utilities|Array|Get(acopy) _outactors_3))
      (Variables|Default|Setplayer1Turn false)
      (bind _asplayer_1_2 (Utilities|Casting|CastToplayer1 (Game|Player|GetPlayerPawn 0)))
      (Variables|/Game/FirstPersonBP/Blueprints/player1.player1_C|Setspacesleft _asplayer_1_2 3)
      (else
        (bind _outactors_4 (Actor|GetAllActorsOfClass "/Game/FirstPersonBP/Blueprints/player2.player2_C"))
        (Pawn|Possess (Utilities|Array|Get(acopy) _outactors_4))
        (Variables|Default|Setplayer1Turn true)
        (bind _asplayer_2_2 (Utilities|Casting|CastToplayer2 (Game|Player|GetPlayerPawn 0)))
        (Variables|/Game/FirstPersonBP/Blueprints/player2.player2_C|Setspacesleft _asplayer_2_2 3)))
    (Variables|Default|SetplaneCurrentPlace 0)
    (bind _outactors_5 (Actor|GetAllActorsOfClass "/Game/plane.plane_C"))
    (Variables|/Game/plane.plane_C|Setdirection%20to%20leave (Utilities|Array|Get(acopy) _outactors_5 (Variables|Default|GetplaneCurrentPlace)) "null" :!label _label)
    (Variables|/Game/plane.plane_C|Setway%20the%20player%20came%20in (Utilities|Array|Get(acopy) _outactors_5 (Variables|Default|GetplaneCurrentPlace)) "null")
    (if (not (== (Variables|Default|GetplaneCurrentPlace) (Utilities|Array|Length _outactors_5)))
      (Math|Integer|IncrementInt (Variables|Default|GetplaneCurrentPlace)
        (:%20%20
          (goto _label))))))

(fn ConstructionScript)

(fn Test
  (if (Variables|Default|Getplayer1Turn)
    (bind _outactors (Actor|GetAllActorsOfClass "/Game/FirstPersonBP/Blueprints/player1.player1_C"))
    (Pawn|Possess (Utilities|Array|Get(acopy) _outactors))
    (Variables|Default|Setplayer1Turn false)
    (bind _asplayer_1 (Utilities|Casting|CastToplayer1 (Game|Player|GetPlayerPawn 0)))
    (Variables|/Game/FirstPersonBP/Blueprints/player1.player1_C|Setspacesleft _asplayer_1 3)
    (else
      (bind _outactors_2 (Actor|GetAllActorsOfClass "/Game/FirstPersonBP/Blueprints/player2.player2_C"))
      (Pawn|Possess (Utilities|Array|Get(acopy) _outactors_2))
      (Variables|Default|Setplayer1Turn true)
      (bind _asplayer_2 (Utilities|Casting|CastToplayer2 (Game|Player|GetPlayerPawn 0)))
      (Variables|/Game/FirstPersonBP/Blueprints/player2.player2_C|Setspacesleft _asplayer_2 3))))